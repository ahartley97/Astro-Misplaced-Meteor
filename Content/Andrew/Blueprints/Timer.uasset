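; Countdown-style timer Blueprint that runs a timeline, publishes its value as OutputedTime and sets TimerFinished when it ends.
; BeginPlay starts the timeline, and Tick polls a Restart flag to reset it and play from the start.
; Each timeline update also looks up the NewBlueprint2 actor, then enlarges and lowers its sphere by fixed increments, so that motion depends on frame rate.
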(event Custom|Starting%20time
  (bind _newtrack_0 (Timeline|Timeline_0 SetNewTime)
    (:Update
      (bind _returnvalue (Actor|GetActorOfClass "/Game/Andrew/Blueprints/NewBlueprint2.NewBlueprint2_C"))
      (Variables|Default|SetOutputed%20Time _newtrack_0)
      (Transformation|SetWorldScale3D (Variables|/Game/Andrew/Blueprints/NewBlueprint2.NewBlueprint2_C|GetSphere _returnvalue) (Math|Vector|MakeVector (+ (.x (Transformation|GetWorldScale (Variables|/Game/Andrew/Blueprints/NewBlueprint2.NewBlueprint2_C|GetSphere _returnvalue))) 0.01) (+ (.y (Transformation|GetWorldScale (Variables|/Game/Andrew/Blueprints/NewBlueprint2.NewBlueprint2_C|GetSphere _returnvalue))) 0.01) (+ (.z (Transformation|GetWorldScale (Variables|/Game/Andrew/Blueprints/NewBlueprint2.NewBlueprint2_C|GetSphere _returnvalue))) 0.01)))
      (Transformation|SetWorldLocation (Variables|/Game/Andrew/Blueprints/NewBlueprint2.NewBlueprint2_C|GetSphere _returnvalue) (Math|Vector|MakeVector (.x (Transformation|GetWorldLocation (Variables|/Game/Andrew/Blueprints/NewBlueprint2.NewBlueprint2_C|GetSphere _returnvalue))) (.y (Transformation|GetWorldLocation (Variables|/Game/Andrew/Blueprints/NewBlueprint2.NewBlueprint2_C|GetSphere _returnvalue))) (+ (.z (Transformation|GetWorldLocation (Variables|/Game/Andrew/Blueprints/NewBlueprint2.NewBlueprint2_C|GetSphere _returnvalue))) -0.35)) false false))
    (:Finished
      (Variables|Default|SetTimerFinished true))))

(event EventTick
  (params (DeltaSeconds :type Float%20%28single-precision%29))
  (if (Variables|Default|GetRestart)
    (CallFunction|StartingTime)
    (Variables|Default|SetRestart false)
    (bind _newtrack_0 (Timeline|Timeline_0 PlayFromStart)
      (:Update
        (bind _returnvalue (Actor|GetActorOfClass "/Game/Andrew/Blueprints/NewBlueprint2.NewBlueprint2_C"))
        (Variables|Default|SetOutputed%20Time _newtrack_0)
        (Transformation|SetWorldScale3D (Variables|/Game/Andrew/Blueprints/NewBlueprint2.NewBlueprint2_C|GetSphere _returnvalue) (Math|Vector|MakeVector (+ (.x (Transformation|GetWorldScale (Variables|/Game/Andrew/Blueprints/NewBlueprint2.NewBlueprint2_C|GetSphere _returnvalue))) 0.01) (+ (.y (Transformation|GetWorldScale (Variables|/Game/Andrew/Blueprints/NewBlueprint2.NewBlueprint2_C|GetSphere _returnvalue))) 0.01) (+ (.z (Transformation|GetWorldScale (Variables|/Game/Andrew/Blueprints/NewBlueprint2.NewBlueprint2_C|GetSphere _returnvalue))) 0.01)))
        (Transformation|SetWorldLocation (Variables|/Game/Andrew/Blueprints/NewBlueprint2.NewBlueprint2_C|GetSphere _returnvalue) (Math|Vector|MakeVector (.x (Transformation|GetWorldLocation (Variables|/Game/Andrew/Blueprints/NewBlueprint2.NewBlueprint2_C|GetSphere _returnvalue))) (.y (Transformation|GetWorldLocation (Variables|/Game/Andrew/Blueprints/NewBlueprint2.NewBlueprint2_C|GetSphere _returnvalue))) (+ (.z (Transformation|GetWorldLocation (Variables|/Game/Andrew/Blueprints/NewBlueprint2.NewBlueprint2_C|GetSphere _returnvalue))) -0.35)) false false))
      (:Finished
        (Variables|Default|SetTimerFinished true)))))

(event EventBeginPlay
  (CallFunction|StartingTime)
  (bind _newtrack_0 (Timeline|Timeline_0 Play)
    (:Update
      (bind _returnvalue (Actor|GetActorOfClass "/Game/Andrew/Blueprints/NewBlueprint2.NewBlueprint2_C"))
      (Variables|Default|SetOutputed%20Time _newtrack_0)
      (Transformation|SetWorldScale3D (Variables|/Game/Andrew/Blueprints/NewBlueprint2.NewBlueprint2_C|GetSphere _returnvalue) (Math|Vector|MakeVector (+ (.x (Transformation|GetWorldScale (Variables|/Game/Andrew/Blueprints/NewBlueprint2.NewBlueprint2_C|GetSphere _returnvalue))) 0.01) (+ (.y (Transformation|GetWorldScale (Variables|/Game/Andrew/Blueprints/NewBlueprint2.NewBlueprint2_C|GetSphere _returnvalue))) 0.01) (+ (.z (Transformation|GetWorldScale (Variables|/Game/Andrew/Blueprints/NewBlueprint2.NewBlueprint2_C|GetSphere _returnvalue))) 0.01)))
      (Transformation|SetWorldLocation (Variables|/Game/Andrew/Blueprints/NewBlueprint2.NewBlueprint2_C|GetSphere _returnvalue) (Math|Vector|MakeVector (.x (Transformation|GetWorldLocation (Variables|/Game/Andrew/Blueprints/NewBlueprint2.NewBlueprint2_C|GetSphere _returnvalue))) (.y (Transformation|GetWorldLocation (Variables|/Game/Andrew/Blueprints/NewBlueprint2.NewBlueprint2_C|GetSphere _returnvalue))) (+ (.z (Transformation|GetWorldLocation (Variables|/Game/Andrew/Blueprints/NewBlueprint2.NewBlueprint2_C|GetSphere _returnvalue))) -0.35)) false false))
    (:Finished
      (Variables|Default|SetTimerFinished true))))

(fn ConstructionScript)
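; Oxygen tank actor that cycles between inactive and active, flagging players inside its sphere as in health range while active.
; A timeline serves as the inactive interval, then the O2_Shutter sequence plays during the active phase and restarts the timeline when finished.
; Tick toggles visibility, adding a new Oxygen widget every active frame and removing all when inactive.
; HealthRange is set only on overlap begin and cleared on exit.
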(event OnComponentEndOverlap(Sphere)
  (params (OverlappedComponent :type Primitive%20Component%20Object%20Reference) (OtherActor :type Actor%20Object%20Reference) (OtherComp :type Primitive%20Component%20Object%20Reference) (OtherBodyIndex :type Integer))
  (bind _asplayer_char (Utilities|Casting|CastToPlayer_Char OtherActor))
  (Variables|/Game/Dylan/Player/Player_Char.Player_Char_C|SetHealthRange _asplayer_char false))

(event OnComponentBeginOverlap(Sphere)
  (params (OverlappedComponent :type Primitive%20Component%20Object%20Reference) (OtherActor :type Actor%20Object%20Reference) (OtherComp :type Primitive%20Component%20Object%20Reference) (OtherBodyIndex :type Integer) (bFromSweep :type Boolean) (SweepResult :type Hit%20Result%20Structure%20%28by%20ref%29))
  (bind _asplayer_char (Utilities|Casting|CastToPlayer_Char OtherActor))
  (if (Variables|Default|GetActive)
    (Variables|/Game/Dylan/Player/Player_Char.Player_Char_C|SetHealthRange _asplayer_char true)))

(event Custom|OnFinished_Event_0
  (Variables|Default|SetActive false)
  (Timeline|Timeline_0 PlayFromStart
    (:Finished
      (bind _returnvalue (Sequencer|Player|CreateLevelSequencePlayer "/Game/Dylan/O2_Shutter.O2_Shutter"))
      (Sequencer|Player|Play _returnvalue :!class /Script/MovieScene.MovieSceneSequencePlayer)
      (Variables|Default|SetActive true)
      (EventDispatchers|AssignOnFinished _returnvalue (delegate Custom|OnFinished_Event_0)))))

(event EventTick
  (params (DeltaSeconds :type Float%20%28single-precision%29))
  (if (Variables|Default|GetActive)
    (Rendering|SetActorHiddenInGame false)
    (bind _returnvalue (UserInterface|CreateWidget "/Game/Andrew/HUDs/Oxygen.Oxygen_C"))
    (UserInterface|Viewport|AddtoViewport _returnvalue 0)
    (else
      (Rendering|SetActorHiddenInGame true)
      (bind _foundwidgets (Widget|GetAllWidgetsOfClass "/Game/Andrew/HUDs/Oxygen.Oxygen_C" true))
      (for _array_element _foundwidgets
        (Widget|RemovefromParent _array_element)))))

(event EventBeginPlay
  (Timeline|Timeline_0 Play
    (:Finished
      (bind _returnvalue (Sequencer|Player|CreateLevelSequencePlayer "/Game/Dylan/O2_Shutter.O2_Shutter"))
      (Sequencer|Player|Play _returnvalue :!class /Script/MovieScene.MovieSceneSequencePlayer)
      (Variables|Default|SetActive true)
      (EventDispatchers|AssignOnFinished _returnvalue (delegate Custom|OnFinished_Event_0)))))

(fn ConstructionScript)
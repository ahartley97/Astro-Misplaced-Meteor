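; Rock spawner where the player picks up rocks of a random size from 1 to 3, rolled at BeginPlay.
; The Sphere1 overlap flags the player as in range and passes the size to TEMPRockSize when they hold no rock.
; Tick polls the player's HasRock, showing Sphere while empty-handed.
; Once a rock is held, a latch hides it, rerolls the size and updates TEMPRockSize once.
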(event OnComponentBeginOverlap(Sphere1)
  (params (OverlappedComponent :type Primitive%20Component%20Object%20Reference) (OtherActor :type Actor%20Object%20Reference) (OtherComp :type Primitive%20Component%20Object%20Reference) (OtherBodyIndex :type Integer) (bFromSweep :type Boolean) (SweepResult :type Hit%20Result%20Structure%20%28by%20ref%29))
  (bind _asplayer_char (Utilities|Casting|CastToPlayer_Char OtherActor))
  (Variables|/Game/Dylan/Player/Player_Char.Player_Char_C|SetRockRange _asplayer_char true)
  (if (not (Variables|/Game/Dylan/Player/Player_Char.Player_Char_C|GetHasRock? _asplayer_char))
    (Variables|Default|SetHUD%20Active true)
    (Variables|/Game/Dylan/Player/Player_Char.Player_Char_C|SetTEMPRockSize _asplayer_char (Math|Float|Truncate (Variables|Default|GetSizeOfRock)))))

(event OnComponentEndOverlap(Sphere1)
  (params (OverlappedComponent :type Primitive%20Component%20Object%20Reference) (OtherActor :type Actor%20Object%20Reference) (OtherComp :type Primitive%20Component%20Object%20Reference) (OtherBodyIndex :type Integer))
  (bind _asplayer_char (Utilities|Casting|CastToPlayer_Char OtherActor))
  (Variables|/Game/Dylan/Player/Player_Char.Player_Char_C|SetRockRange _asplayer_char false)
  (if (Variables|Default|GetHUD%20Active)
    (Variables|/Game/Dylan/Player/Player_Char.Player_Char_C|SetTEMPRockSize _asplayer_char 0)))

(event Custom|newrock
  (Variables|Default|SetSizeOfRock (Math|Conversions|ToFloat(Integer) (Math|Random|RandomIntegerinRange 1 3))))

(event EventTick
  (params (DeltaSeconds :type Float%20%28single-precision%29))
  (bind _asplayer_char (Utilities|Casting|CastToPlayer_Char (Game|GetPlayerCharacter 0)))
  (if (not (Variables|/Game/Dylan/Player/Player_Char.Player_Char_C|GetHasRock? _asplayer_char))
    (Rendering|SetVisibility (Variables|Default|GetSphere) true false)
    (Variables|Default|SetNewVar_0 true)
    (elif (Variables|Default|GetNewVar_0)
      (Rendering|SetVisibility (Variables|Default|GetSphere) false false)
      (CallFunction|Newrock)
      (Variables|Default|SetNewVar_0 false)
      (Variables|/Game/Dylan/Player/Player_Char.Player_Char_C|SetTEMPRockSize _asplayer_char (Math|Float|Truncate (Variables|Default|GetSizeOfRock))))))

(event EventBeginPlay
  (CallFunction|Newrock))

(fn ConstructionScript)